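; InputPawn is a pawn that drives two player paddles (P1 and P2) from separate vertical input axes.
; Each axis event moves its paddle along world Z, scaled by a shared paddle speed variable and frame delta time.
; Movement uses swept world offsets, so the paddles collide with blocking geometry instead of passing through it.
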(event EventBeginPlay)

(event Collision|EventActorBeginOverlap
  (params (OtherActor :type Actor%20Object%20Reference)))

(event EventTick
  (params (DeltaSeconds :type Float%20%28single-precision%29)))

(event Input|AxisEvents|InputAxisP1_Cima
  (params (AxisValue :type Float%20%28single-precision%29))
  ;[1 1 1] Movimentação P1
  (Transformation|AddActorWorldOffset (Variables|Default|GetP1) (Math|Vector|MakeVector 0.0 0.0 (* (* AxisValue (Variables|Default|GetVelocidadeRaquete)) (Utilities|Time|GetWorldDeltaSeconds))) true))

(event Input|AxisEvents|InputAxisP2_Cima
  (params (AxisValue :type Float%20%28single-precision%29))
  ;[1 1 1] Movimentação P2
  (Transformation|AddActorWorldOffset (Variables|Default|GetP2) (Math|Vector|MakeVector 0.0 0.0 (* (* AxisValue (Variables|Default|GetVelocidadeRaquete)) (Utilities|Time|GetWorldDeltaSeconds))) true))

(fn ConstructionScript)