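; Ball actor for a Pong game that moves itself every tick with a swept world offset and reacts to whatever it hits.
; Paddle hits reverse X, set Z from the impact height relative to the paddle centre and speed the ball up.
; Goal hits reset position and speed, reverse X and add score through PongGameMode; other hits flip Z.
; Each blocking hit also triggers a camera shake and sparks.
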(event EventBeginPlay)

(event Collision|EventActorBeginOverlap
  (params (OtherActor :type Actor%20Object%20Reference)))

(event EventTick
  (params (DeltaSeconds :type Float%20%28single-precision%29))
  (bind _sweephitresult (Transformation|AddActorWorldOffset (* (Variables|Default|GetDirecao) (* DeltaSeconds (Variables|Default|GetVelocidade))) true))
  (if (.bBlockingHit (Collision|BreakHitResult _sweephitresult))
    (Utilities|FlowControl|Sequence
      (:then_0
        ;[1 1 1] Bola batendo nas raquetes
        (if (Actor|ActorHasTag (.HitActor (Collision|BreakHitResult _sweephitresult)) "Raquete")
          (Utilities|FlowControl|Sequence
            (:then_0
              (bind _z (CallFunction|VariarDirecaoBola (.Location (Collision|BreakHitResult _sweephitresult)) (Transformation|GetActorLocation (.HitActor (Collision|BreakHitResult _sweephitresult)))))
              (Variables|Default|SetDirecao (Math|Vector|MakeVector (* (.X (Math|Vector|BreakVector (Variables|Default|GetDirecao))) -1.0) (.Y (Math|Vector|BreakVector (Variables|Default|GetDirecao))) _z))
              (Audio|PlaySound2D "/Game/Assets/Audio/HitSound.HitSound" 1.0 1.0 0.0 0 0))
            (:then_1
              (Variables|Default|SetVelocidade (* (Variables|Default|GetVelocidade) 1.06))))
          (else
            ;[1 1 1] Pontuação
            (if (Actor|ActorHasTag (.HitActor (Collision|BreakHitResult _sweephitresult)) "Pontuacao")
              (Transformation|SetActorLocation "0, 0, 0" false true)
              (Utilities|FlowControl|Sequence
                (:then_0
                  (Variables|Default|SetDirecao (Math|Vector|MakeVector (* (.X (Math|Vector|BreakVector (Variables|Default|GetDirecao))) -1.0) (.Y (Math|Vector|BreakVector (Variables|Default|GetDirecao))) (.Z (Math|Vector|BreakVector (Variables|Default|GetDirecao)))))
                  (bind _aspontuacao_actor (Utilities|Casting|CastToPontuacaoActor (.HitActor (Collision|BreakHitResult _sweephitresult))))
                  (bind _aspong_game_mode (Utilities|Casting|CastToPongGameMode (Game|GetGameMode)))
                  (Default|AddScore _aspong_game_mode (Variables|/Game/Blueprints/PontuacaoActor.PontuacaoActor_C|GetPlayerIndex _aspontuacao_actor))
                  (Audio|PlaySound2D "/Game/Assets/Audio/ScoreSound.ScoreSound" 1.0 1.0 0.0 0 0))
                (:then_1
                  (Variables|Default|SetVelocidade 2.2e+02)))
              (else
                ;[1 1 1] Bola batendo nos limites
                (Variables|Default|SetDirecao (Math|Vector|MakeVector (.X (Math|Vector|BreakVector (Variables|Default|GetDirecao))) (.Y (Math|Vector|BreakVector (Variables|Default|GetDirecao))) (* (.Z (Math|Vector|BreakVector (Variables|Default|GetDirecao))) -1.0)))
                (Audio|PlaySound2D "/Game/Assets/Audio/HitSound.HitSound" 1.0 1.0 0.0 0 0))))))
      (:then_1
        (Camera|PlayWorldCameraShake "/Game/Blueprints/PongCameraShake.PongCameraShake_C" "0, 0, 0" 0.0 5e+04)
        (Effects|SpawnEmitteratLocation "/Game/Assets/Particles/SparkParticleSystem.SparkParticleSystem" (.Location (Collision|BreakHitResult _sweephitresult)))))))

(fn ConstructionScript)

(fn VariarDirecaoBola
  (params (LocalizacaoColisao :type Vector) (LocalizacaoRaquete :type Vector))
  (return (/ (- (.Z (Math|Vector|BreakVector LocalizacaoColisao)) (.Z (Math|Vector|BreakVector LocalizacaoRaquete))) 45.0)))