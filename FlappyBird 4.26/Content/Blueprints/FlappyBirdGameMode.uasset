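; Game mode for a Flappy Bird style game that owns the score HUD and broadcasts game state changes.
; On BeginPlay it creates the score widget and adds it to the viewport.
; NotifyGameStarted and NotifyGameEnded find every actor implementing GameStateInterface and send it the matching start or end message.
; The Pontuação function increments the player's score counter.
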(event EventBeginPlay
  (bind _returnvalue (UserInterface|CreateWidget "/Game/Blueprints/ScoreWidget.ScoreWidget_C"))
  (bind _output_get (Variables|Default|SetFlappyWidget _returnvalue))
  (UserInterface|Viewport|AddtoViewport _output_get 0))

(event EventTick
  (params (DeltaSeconds :type Float%20%28single-precision%29)))

(fn ConstructionScript)

(fn NotifyGameStarted
  (bind _outactors (Actor|GetAllActorswithInterface "/Game/Blueprints/GameStateInterface.GameStateInterface_C"))
  (for _array_element _outactors
    (Class|GameStateInterface|GameStarted(Message) _array_element)))

(fn NotifyGameEnded
  (bind _outactors (Actor|GetAllActorswithInterface "/Game/Blueprints/GameStateInterface.GameStateInterface_C"))
  (for _array_element _outactors
    (Class|GameStateInterface|GameEnded(Message) _array_element)))

(fn Pontuação
  (bind _result (Math|Integer|IncrementInt (Variables|Default|GetScorePlayer))
    (:%20%20
      (Variables|Default|SetScorePlayer _result))))