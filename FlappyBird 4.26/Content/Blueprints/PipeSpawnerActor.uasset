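; Pipe spawner actor that periodically spawns pipe obstacles while the game runs.
; The GameStarted event spawns a pipe immediately, then starts a looping timer that repeats SpawnPipe at a fixed interval; GameEnded clears it.
; SpawnPipe creates a PipeClass actor at the spawner's X and Y position, with a random height within a fixed range.
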(event EventBeginPlay)

(event Collision|EventActorBeginOverlap
  (params (OtherActor :type Actor%20Object%20Reference)))

(event EventTick
  (params (DeltaSeconds :type Float%20%28single-precision%29)))

(event EventGameStarted
  (CallFunction|SpawnPipe)
  (bind _returnvalue (Utilities|Time|SetTimerbyFunctionName 0 "SpawnPipe" 2.6 true))
  (Variables|Default|SetTimerHandle _returnvalue))

(event EventGameEnded
  (Utilities|Time|ClearandInvalidateTimerbyHandle (Variables|Default|GetTimerHandle)))

(fn ConstructionScript)

(fn SpawnPipe
  (bind _returnvalue (Transformation|GetActorLocation))
  (Game|SpawnActorfromClass (Variables|Default|GetPipeClass) (Math|Transform|MakeTransform (Math|Vector|MakeVector (.x _returnvalue) (.y _returnvalue) (Math|Random|RandomFloatinRange -6e+01 1.6e+02)) "0, 0, 0" "1,1,1") "Undefined" 0 0))