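; Player bird pawn for a Flappy Bird clone, handling flapping, scoring, death and level restart.
; While playing, Tick applies manual gravity through a swept world offset and tilts the flipbook by vertical velocity.
; The first flap starts the game through FlappyBirdGameMode, and each flap resets upward speed.
; Sphere overlaps score on ScoreBox-tagged components; any other marks the bird dead and notifies the game mode.
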(event OnComponentBeginOverlap(Sphere)
  (params (OverlappedComponent :type Primitive%20Component%20Object%20Reference) (OtherActor :type Actor%20Object%20Reference) (OtherComp :type Primitive%20Component%20Object%20Reference) (OtherBodyIndex :type Integer) (bFromSweep :type Boolean) (SweepResult :type Hit%20Result%20Structure%20%28by%20ref%29))
  (if (Components|ComponentHasTag OtherComp "ScoreBox")
    (bind _asflappy_bird_game_mode (Utilities|Casting|CastToFlappyBirdGameMode (Game|GetGameMode)))
    (Default|Pontuação _asflappy_bird_game_mode)
    (Audio|PlaySound2D "/Game/Asstes/Sound/Ponto.Ponto" 1.0 1.0 0.0 0 0)
    (else
      (Variables|Default|SetIsDead true)
      (bind _asflappy_bird_game_mode_2 (Utilities|Casting|CastToFlappyBirdGameMode (Game|GetGameMode)))
      (Default|NotifyGameEnded _asflappy_bird_game_mode_2)
      (Utilities|FlowControl|DoOnce false
        (:Completed
          (Audio|PlaySound2D "/Game/Asstes/Sound/Morreu.Morreu" 1.0 1.0 0.0 0 0))))))

(event EventBeginPlay)

(event Collision|EventActorBeginOverlap
  (params (OtherActor :type Actor%20Object%20Reference)))

(event EventTick
  (params (DeltaSeconds :type Float%20%28single-precision%29))
  (if (Variables|Default|GetIsPlaying)
    (bind _output_get (Variables|Default|SetDirection (Math|Vector|MakeVector (.x (Variables|Default|GetDirection)) (.y (Variables|Default|GetDirection)) (+ (.z (Variables|Default|GetDirection)) (* DeltaSeconds (Variables|Default|GetGravity))))))
    (Transformation|AddActorWorldOffset _output_get true)
    (Transformation|SetRelativeRotation (Variables|Default|GetPaperFlipbook) (Math|Rotator|Lerp(Rotator) "-60.000000, 0, 0" "30.000000, 0, 0" (Math|Float|Clamp(Float) (/ (+ (.z (Variables|Default|GetDirection)) 2.0) 3.0))) false false)))

(event Input|ActionEvents|InputActionFlap
  (params (Key :type Key%20Structure :default "None"))
  (:Pressed
    (if (not (Variables|Default|GetIsDead))
      (if (Variables|Default|GetIsPlaying)
        _
        (else
          (bind _asflappy_bird_game_mode (Utilities|Casting|CastToFlappyBirdGameMode (Game|GetGameMode)))
          (Default|NotifyGameStarted _asflappy_bird_game_mode)
          (Variables|Default|SetIsPlaying true)))
      (Variables|Default|SetDirection (Math|Vector|MakeVector (.x (Variables|Default|GetDirection)) (.y (Variables|Default|GetDirection)) (Variables|Default|GetFlapSpeed)))
      (Audio|PlaySound2D "/Game/Asstes/Sound/Voo.Voo" 1.0 1.0 0.0 0 0))))

(event Input|ActionEvents|InputActionRestartGame
  (params (Key :type Key%20Structure :default "None"))
  (:Pressed
    (Game|OpenLevel(byName) "Game"))
  (:Released
    (Audio|PlaySound2D "/Game/Asstes/Sound/Restart.Restart" 1.0 1.0 0.0 0 0)))

(fn ConstructionScript)